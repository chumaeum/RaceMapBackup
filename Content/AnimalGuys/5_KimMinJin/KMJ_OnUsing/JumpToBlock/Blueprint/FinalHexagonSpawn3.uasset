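; Spawner actor that builds part of a hexagon layout, likely for the JumpToBlock minigame, by placing HexagonSpawn11 actors.
; On BeginPlay a loop computes each position from its index, stepping along X with offsets on X and Y derived from half the index.
; Each spawned actor is attached to this actor with Keep Relative rules, so the computed positions act as local offsets.
; A disconnected FlipFlop spawn branch never runs.
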(event `self.ReceiveBeginPlay`
  (set `self.location` (`self.K2_GetActorLocation`))
  (for _index (range 11)
    (bind _returnvalue (/ _index 2))
    (bind _output_get (set `self.location` (`KismetMathLibrary.MakeVector` (+ (* _index 170.0) (* _returnvalue -80.0)) (* _returnvalue -150.0))))
    (bind _returnvalue_2 (`|SpawnActorFromClass` "/Game/AnimalGuys/5_KimMinJin/KMJ_OnUsing/JumpToBlock/Blueprint/HexagonSpawn1-1.HexagonSpawn1-1_C" (`KismetMathLibrary.MakeTransform` _output_get) "Undefined" "OverrideRootScale" null null))
    (`self.K2_AttachToActor` _returnvalue_2 self "None" "KeepRelative" "KeepRelative" "KeepRelative" true)))

(fn `UserConstructionScript`)